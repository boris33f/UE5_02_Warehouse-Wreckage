(fn ConstructionScript)

(fn PrintYourName
  (Development|PrintString (Utilities|GetDisplayName self)))

(fn Launch
  (bind _self self)
  (Physics|AddImpulse (Variables|/Script/Engine.StaticMeshActor|GetStaticMeshComponent _self) (* (Math|Vector|GetForwardVector (Math|Transform|TransformRotation (Transformation|GetActorTransform _self) "0, 0, 0")) 2000000) "None" false))